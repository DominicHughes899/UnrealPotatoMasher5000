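; Player character Blueprint for the Potato Masher that shows a progress bar during timed interactions.
; On BeginPlay it caches the WBP_InteractionProgressBar from its Widget component, hides it and turns off the component's shadow casting.
; Interaction begin and end events toggle the bar's visibility, and timer updates feed the completion percent into it.
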(event EventBeginPlay
  (bind _aswbp_interaction_progress_bar (Utilities|Casting|CastToWBP_InteractionProgressBar (UserInterface|GetWidget (Variables|Default|GetWidget))))
  (bind _output_get (Variables|Default|SetProgressWidget _aswbp_interaction_progress_bar))
  (Widget|SetVisibility _output_get "Hidden")
  (Rendering|SetCastShadow (Variables|Default|GetWidget) false))

(event EventOnBeginInteraction
  ;[1 1 1] Action timer widget functions
  (Widget|SetVisibility (Variables|Default|GetProgressWidget) "Visible"))

(event EventOnEndInteraction
  ;[1 1 1] Action timer widget functions
  (Widget|SetVisibility (Variables|Default|GetProgressWidget) "Hidden"))

(event EventOnUpdateTimer
  (params (CompletionPercent :type Float%20%28single-precision%29))
  ;[1 1 1] Action timer widget functions
  (Default|SetPercent (Variables|Default|GetProgressWidget) CompletionPercent))

(fn ConstructionScript)