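; Player controller that creates the main HUD overlay and feeds it delivery-style contracts, each with a package type, required quantity and reward.
; On BeginPlay it adds WBP_MainOverlay to the viewport and seeds it with a fixed diced-carrot contract.
; Tab or the gamepad left shoulder toggles the contracts panel, while T adds a diced-carrot contract with random quantity and reward.
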(event EventBeginPlay
  (bind _returnvalue (UserInterface|CreateWidget "/Game/Core/UI/Overlay/WBP_MainOverlay.WBP_MainOverlay_C"))
  (bind _output_get (Variables|Default|SetMainOverlay _returnvalue))
  (UserInterface|Viewport|AddtoViewport _output_get 0)
  (Default|AddContract (Variables|Default|GetMainOverlay) (Utilities|Struct|MakeContractStruct "DicedCarrots" 15 0 500)))

(event Input|GamepadEvents|GamepadLeftShoulder
  (params (Key :type Key%20Structure :default "None"))
  (:Pressed
    (Default|OpenCloseContracts (Variables|Default|GetMainOverlay))))

(event Input|KeyboardEvents|T
  (params (Key :type Key%20Structure :default "None"))
  (:Pressed
    (Default|AddContract (Variables|Default|GetMainOverlay) (Utilities|Struct|MakeContractStruct "DicedCarrots" (Math|Random|RandomInteger 20) 0 (Math|Random|RandomIntegerinRange 100 500)))))

(event Input|KeyboardEvents|Tab
  (params (Key :type Key%20Structure :default "None"))
  (:Pressed
    (Default|OpenCloseContracts (Variables|Default|GetMainOverlay))))

(fn ConstructionScript)